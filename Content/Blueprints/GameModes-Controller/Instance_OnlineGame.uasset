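; Game instance Blueprint that hosts and joins online multiplayer sessions.
; HostSession builds a random two-word server name and four-part password from arrays, then creates an advanced session carrying them, visibility and round count as extra settings.
; Successful hosting opens the lobby map as a listen server.
; Failures create error widgets, though only the hosting one is added to the viewport.
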(event `JoinSession`
  (params (Session :type "BlueprintSessionResult Structure (by ref)"))
  (`JoinSessionCallbackProxy.JoinSession` (`GameplayStatics.GetPlayerController` 0) Session
    (:`OnFailure`
      (`|CreateWidget` "/Game/Networking/Widgets/Widget_ErrorMessage.Widget_ErrorMessage_C" null "Failed to join session"))))

(event `HostSession`
  (params (NumberOfPlayersPerSession :type Integer))
  (bind _firstwordarray (`self.FirstWordArray`))
  (bind _secondwordarray (`self.SecondWordArray`))
  (bind _passwordletter_1 (`self.PasswordLetter_1`))
  (bind _passwordletter_2 (`self.PasswordLetter_2`))
  (bind _passwordletter_3 (`self.PasswordLetter_3`))
  (bind _passwordletter_4 (`self.PasswordLetter_4`))
  (bind _output_get (set `self.SessionTitleResult` (`|FormatText` "{a} {b}" (`self.Random Array Choice` _firstwordarray _firstwordarray) (`self.Random Array Choice` _secondwordarray _secondwordarray))))
  (bind _output_get_2 (set `self.PasswordOutput` (`|FormatText` "{a}{b}{c}{d}" (`self.Random Array Choice` _passwordletter_1 _passwordletter_1) (`self.Random Array Choice` _passwordletter_2 _passwordletter_2) (`self.Random Array Choice` _passwordletter_3 _passwordletter_3) (`self.Random Array Choice` _passwordletter_4 _passwordletter_4))))
  (bind _output_get_3 (set `self.Number Of Players Per Session` NumberOfPlayersPerSession))
  (`CreateSessionCallbackProxyAdvanced.CreateAdvancedSession` (`|MakeArray` (`AdvancedSessionsLibrary.MakeLiteralSessionPropertyString` "ServerName" (`KismetTextLibrary.Conv_TextToString` _output_get)) (`AdvancedSessionsLibrary.MakeLiteralSessionPropertyString` "ServerPassword" (`KismetTextLibrary.Conv_TextToString` _output_get_2)) (`AdvancedSessionsLibrary.MakeLiteralSessionPropertyString` "PublicOrPrivate" (`KismetTextLibrary.Conv_TextToString` (`self.PublicOrPrivate`))) (`AdvancedSessionsLibrary.MakeLiteralSessionPropertyString` "NumberOfRounds" (`KismetStringLibrary.Conv_IntToString` (`self.Rounds`)))) (`GameplayStatics.GetPlayerController` 0) _output_get_3
    (:`OnSuccess`
      (`GameplayStatics.OpenLevelBySoftObjectPtr` "/Game/Maps/Map_LobbyLevel.Map_LobbyLevel" true "listen"))
    (:`OnFailure`
      (bind _returnvalue (`|CreateWidget` "/Game/Networking/Widgets/Widget_ErrorMessage.Widget_ErrorMessage_C" null "Failed to make session"))
      (`UserWidget.AddToViewport` _returnvalue 0))))