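; Main game camera pawn that lays out a set of cards when play begins.
; Empty scene components on the pawn act as ten card slots.
; BeginPlay spawns an Actor_Card_Movement at each slot's world transform, one hardcoded call per slot, as placeholder logic.
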(event `self.ReceiveBeginPlay`
  (`|SpawnActorFromClass` "/Game/Networking/Actor_Card_Movement.Actor_Card_Movement_C" (`SceneComponent.K2_GetComponentToWorld` (`self.CardSlot_1`)) "Undefined" "OverrideRootScale" null null)
  (`|SpawnActorFromClass` "/Game/Networking/Actor_Card_Movement.Actor_Card_Movement_C" (`SceneComponent.K2_GetComponentToWorld` (`self.CardSlot_2`)) "Undefined" "OverrideRootScale" null null)
  (`|SpawnActorFromClass` "/Game/Networking/Actor_Card_Movement.Actor_Card_Movement_C" (`SceneComponent.K2_GetComponentToWorld` (`self.CardSlot_3`)) "Undefined" "OverrideRootScale" null null)
  (`|SpawnActorFromClass` "/Game/Networking/Actor_Card_Movement.Actor_Card_Movement_C" (`SceneComponent.K2_GetComponentToWorld` (`self.CardSlot_4`)) "Undefined" "OverrideRootScale" null null)
  (`|SpawnActorFromClass` "/Game/Networking/Actor_Card_Movement.Actor_Card_Movement_C" (`SceneComponent.K2_GetComponentToWorld` (`self.CardSlot_5`)) "Undefined" "OverrideRootScale" null null)
  (`|SpawnActorFromClass` "/Game/Networking/Actor_Card_Movement.Actor_Card_Movement_C" (`SceneComponent.K2_GetComponentToWorld` (`self.CardSlot_6`)) "Undefined" "OverrideRootScale" null null)
  (`|SpawnActorFromClass` "/Game/Networking/Actor_Card_Movement.Actor_Card_Movement_C" (`SceneComponent.K2_GetComponentToWorld` (`self.CardSlot_7`)) "Undefined" "OverrideRootScale" null null)
  (`|SpawnActorFromClass` "/Game/Networking/Actor_Card_Movement.Actor_Card_Movement_C" (`SceneComponent.K2_GetComponentToWorld` (`self.CardSlot_8`)) "Undefined" "OverrideRootScale" null null)
  (`|SpawnActorFromClass` "/Game/Networking/Actor_Card_Movement.Actor_Card_Movement_C" (`SceneComponent.K2_GetComponentToWorld` (`self.CardSlot_9`)) "Undefined" "OverrideRootScale" null null)
  (`|SpawnActorFromClass` "/Game/Networking/Actor_Card_Movement.Actor_Card_Movement_C" (`SceneComponent.K2_GetComponentToWorld` (`self.CardSlot_10`)) "Undefined" "OverrideRootScale" null null))

(fn `UserConstructionScript`)