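; Game instance that hosts and joins multiplayer sessions, including accepted invites, through Advanced Sessions nodes.
; Hosting builds a random two-word name and four-part password from arrays, then publishes them with privacy and round count as session settings.
; A successful host opens the lobby map as a listen server.
; Failures create an error widget, though only the hosting path adds it to the viewport.
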(event `self.OnSessionInviteAccepted`
  (params (LocalPlayerNum :type Integer) (PersonInvited :type "BPUniqueNetId Structure") (SessionToJoin :type "BlueprintSessionResult Structure (by ref)"))
  (`JoinSessionCallbackProxy.JoinSession` (`GameplayStatics.GetPlayerController` 0) SessionToJoin
    (:`OnFailure`
      (`|CreateWidget` "/Game/Networking/Widgets/Widget_ErrorMessage.Widget_ErrorMessage_C" null "Failed to join session" :!label _label))))

(event `JoinSession`
  (params (Session :type "BlueprintSessionResult Structure (by ref)"))
  (`JoinSessionCallbackProxy.JoinSession` (`GameplayStatics.GetPlayerController` 0) Session
    (:`OnFailure`
      (goto _label))))

(event `HostSession`
  (params (NumberOfPlayersPerSession :type Integer))
  (bind _output_get (set `self.SessionTitleResult` (`|FormatText` "{a} {b}" (`self.Random Array Choice` (`self.FirstWordArray`)) (`self.Random Array Choice` (`self.SecondWordArray`)))))
  (bind _output_get_2 (set `self.PasswordOutput` (`|FormatText` "{a}{b}{c}{d}" (`self.Random Array Choice` (`self.PasswordLetter_1`)) (`self.Random Array Choice` (`self.PasswordLetter_2`)) (`self.Random Array Choice` (`self.PasswordLetter_3`)) (`self.Random Array Choice` (`self.PasswordLetter_4`)))))
  (bind _output_get_3 (set `self.Max Number Of Players Per Session` NumberOfPlayersPerSession))
  (`CreateSessionCallbackProxyAdvanced.CreateAdvancedSession` (`|MakeArray` (`AdvancedSessionsLibrary.MakeLiteralSessionPropertyString` "ServerName" (`KismetTextLibrary.Conv_TextToString` _output_get)) (`AdvancedSessionsLibrary.MakeLiteralSessionPropertyString` "ServerPassword" (`KismetTextLibrary.Conv_TextToString` _output_get_2)) (`AdvancedSessionsLibrary.MakeLiteralSessionPropertyString` "PublicOrPrivate" (`KismetTextLibrary.Conv_TextToString` (`self.PublicOrPrivate`))) (`AdvancedSessionsLibrary.MakeLiteralSessionPropertyString` "NumberOfRounds" (`KismetStringLibrary.Conv_IntToString` (`self.FinalScore`)))) (`GameplayStatics.GetPlayerController` 0) _output_get_3
    (:`OnSuccess`
      (`GameplayStatics.OpenLevelBySoftObjectPtr` "/Game/Maps/Map_LobbyLevel.Map_LobbyLevel" true "listen"))
    (:`OnFailure`
      (bind _returnvalue (`|CreateWidget` "/Game/Networking/Widgets/Widget_ErrorMessage.Widget_ErrorMessage_C" null "Failed to make session"))
      (`UserWidget.AddToViewport` _returnvalue 0))))