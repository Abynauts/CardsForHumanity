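; Main menu monitor actor that shows the Host Game and Join Game screens as widget components.
; Host and join card dispatchers turn on the static screen and bring in the matching widget, with join also running an online FindSessions search to fill the results.
; The game instance's move-to-cards event turns the monitor off and hides both widgets, parking them offscreen so their overlap does not block clicks.
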(event `self.ReceiveBeginPlay`
  (bind _assteam_game_instance (cast `/Game/Blueprints/GameModes-Controller/Steam_GameInstance` (`GameplayStatics.GetGameInstance`)))
  (set `self.Online Game Instance` _assteam_game_instance)
  ;[1 1 1] Sets both widgets offscreen. I need to do this otherwise, they will overlap and you won't be able to click on one.
  (`SceneComponent.K2_SetRelativeLocation` (`self.HostGameWidget`) (500.0 500.0 500.0) false false)
  (`SceneComponent.K2_SetRelativeLocation` (`self.JoinGameWidget`) (500.0 500.0 500.0) false false)
  (bind _returnvalue (`GameplayStatics.GetActorOfClass` "/Game/Blueprints/CardStuff/MainMenuCards/HostGame_Card_Child.HostGame_Card_Child_C"))
  (add `/Game/Blueprints/CardStuff/MainMenuCards/HostGame_Card_Child.Host Camera Move Dispatcher` _returnvalue (delegate `HostCardTransition`))
  (add `/Game/Blueprints/GameModes-Controller/Steam_GameInstance.MoveCameraToCards` (`self.Online Game Instance`) (delegate `MoveToCameraStartTransition`))
  (bind _returnvalue_2 (`GameplayStatics.GetActorOfClass` "/Game/Blueprints/CardStuff/MainMenuCards/JoinGame_Card_Child.JoinGame_Card_Child_C"))
  (add `/Game/Blueprints/CardStuff/MainMenuCards/JoinGame_Card_Child.Join Game Camera Dispatcher` _returnvalue_2 (delegate `JoinCardTransition`)))

(event `ClickedRefreshButton`
  (bind _joingamewidget (`self.JoinGameWidget`))
  (bind _joingamewidget_2 (`self.JoinGameWidget`))
  (bind _aswidget_join_match_screen (cast `/Game/Networking/Widgets/Widget_JoinMatchScreen` (`WidgetComponent.GetWidget` _joingamewidget_2) :!label _label))
  (`SceneComponent.K2_SetRelativeLocation` _joingamewidget_2 (0.0 -10.0 193.0) false false)
  (bind _results (`FindSessionsCallbackProxy.FindSessions` (`GameplayStatics.GetPlayerController` 0) 100)
    (:`OnSuccess`
      (bind _aswidget_join_match_screen_2 (cast `/Game/Networking/Widgets/Widget_JoinMatchScreen` (`WidgetComponent.GetWidget` _joingamewidget)))
      (`/Game/Networking/Widgets/Widget_JoinMatchScreen.PopulateResults` _aswidget_join_match_screen_2 _results)
      (`SceneComponent.SetVisibility` _joingamewidget true false)
      (`/Game/Networking/Widgets/Widget_JoinMatchScreen.TurnOnJoinMatch` _aswidget_join_match_screen)
      (`Widget.SetVisibility` (`/Game/Networking/Widgets/Widget_JoinMatchScreen.Throbber_0` _aswidget_join_match_screen) "Hidden"))))

(event `HostCardTransition`
  (bind _hostgamewidget (`self.HostGameWidget`))
  (`KismetSystemLibrary.Delay` 1.2)
  (bind _aswidget_monitor_static (cast `/Game/Networking/Widgets/Widget_MonitorStatic` (`WidgetComponent.GetWidget` (`self.StaticScreenWidget`))))
  (`/Game/Networking/Widgets/Widget_MonitorStatic.TurnMonitorOn` _aswidget_monitor_static)
  (`KismetSystemLibrary.Delay` 0.8)
  (bind _aswidget_host_game_options (cast `/Game/Networking/Widgets/Widget_HostGameOptions` (`WidgetComponent.GetWidget` _hostgamewidget)))
  (`SceneComponent.SetVisibility` _hostgamewidget true false)
  (`SceneComponent.K2_SetRelativeLocation` _hostgamewidget (0.0 -10.0 170.0) false false)
  (`/Game/Networking/Widgets/Widget_HostGameOptions.TurnOnHostOptions` _aswidget_host_game_options))

(event `JoinCardTransition`
  (`|ExecutionSequence`
    (:`then_0`
      (goto _label))
    (:`then_1`
      (`KismetSystemLibrary.Delay` 1.2)
      (bind _aswidget_monitor_static (cast `/Game/Networking/Widgets/Widget_MonitorStatic` (`WidgetComponent.GetWidget` (`self.StaticScreenWidget`))))
      (`/Game/Networking/Widgets/Widget_MonitorStatic.TurnMonitorOn` _aswidget_monitor_static))))

(event `MoveToCameraStartTransition`
  (bind _hostgamewidget (`self.HostGameWidget`))
  (`|ExecutionSequence`
    (:`then_0`
      (`SceneComponent.SetVisibility` _hostgamewidget false false)
      (`SceneComponent.SetVisibility` (`self.JoinGameWidget`) false false)
      (`SceneComponent.K2_SetRelativeLocation` _hostgamewidget (500.0 500.0 500.0) false false)
      (`SceneComponent.K2_SetRelativeLocation` (`self.JoinGameWidget`) (500.0 500.0 500.0) false false))
    (:`then_1`
      (bind _aswidget_monitor_static (cast `/Game/Networking/Widgets/Widget_MonitorStatic` (`WidgetComponent.GetWidget` (`self.StaticScreenWidget`))))
      (`/Game/Networking/Widgets/Widget_MonitorStatic.TurnMonitorOff` _aswidget_monitor_static))))

(fn `UserConstructionScript`)