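; Main menu player controller that shows a fade-in widget, applies saved options and presents post-game level-up feedback.
; On BeginPlay it loads PlayerOptions to set gamma and master volume, enabling mouse events only if that save exists.
; After a delay, it checks MasterSave for a finished game, shows the level-up widget, adds confetti on level-up, then clears the flag.
; Disconnected achievement, XP and session-notice logic never runs.
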(event `self.ReceiveBeginPlay`
  (bind _returnvalue (`|CreateWidget` "/Game/Blueprints/GameModes-Controller/MainMenu/FadeInWidget.FadeInWidget_C" self))
  (`UserWidget.AddToViewport` _returnvalue 0)
  (`|ExecutionSequence`
    (:`then_0`
      ;[1 1 1] Loads player options if there are any
      (`GameUserSettings.GetGameUserSettings`)
      (bind _returnvalue_2 (`GameplayStatics.DoesSaveGameExist` "PlayerOptions"))
      (if _returnvalue_2
        (bind _returnvalue_3 (`GameplayStatics.LoadGameFromSlot` "PlayerOptions"))
        (bind _assave_data_player_info (cast `/Game/Data/SaveData_PlayerInfo` _returnvalue_3))
        (`KismetSystemLibrary.ExecuteConsoleCommand` (`KismetTextLibrary.Conv_TextToString` (`|FormatText` "Gamma {int}" (`KismetMathLibrary.Round` (`/Game/Data/SaveData_PlayerInfo.Brightness` _assave_data_player_info)))) null)
        (`GameplayStatics.SetSoundMixClassOverride` "/Game/Audio/MasterSoundMix.MasterSoundMix" "/Engine/EngineSounds/Master.Master" (`/Game/Data/SaveData_PlayerInfo.MasterSound` _assave_data_player_info) 1.0 0.0)
        (`GameplayStatics.PushSoundMixModifier` "/Game/Audio/MasterSoundMix.MasterSoundMix")
        (set `self.bEnableClickEvents` true)
        (set `self.bEnableMouseOverEvents` true)))
    (:`then_1`
      (`KismetSystemLibrary.Delay` 2.0)
      (`Widget.RemoveFromParent` _returnvalue)
      (bind _returnvalue_4 (`GameplayStatics.DoesSaveGameExist` "MasterSave"))
      (if _returnvalue_4
        (bind _returnvalue_5 (`GameplayStatics.LoadGameFromSlot` "MasterSave"))
        (bind _assave_data_player_info_2 (cast `/Game/Data/SaveData_PlayerInfo` _returnvalue_5))
        (bind _output_get (set `self.As Save Data Player Info` _assave_data_player_info_2))
        (if (`/Game/Data/SaveData_PlayerInfo.GameEnded` _output_get)
          (set `self.CanActivateCards` false)
          (bind _returnvalue_6 (`|CreateWidget` "/Game/Blueprints/GameModes-Controller/MainMenu/Widget_LevelUp.Widget_LevelUp_C"))
          (`UserWidget.AddToViewport` _returnvalue_6 0)
          (if (`/Game/Data/SaveData_PlayerInfo.LeveledUp` _output_get)
            (`GameplayStatics.SpawnEmitterAtLocation` "/Game/Unlockables/Confetti_P.Confetti_P" (`self.Location_01`) (struct :`Roll` 90.0))
            (`GameplayStatics.SpawnEmitterAtLocation` "/Game/Unlockables/Confetti_P.Confetti_P" (`self.Location_02`) (struct :`Roll` 90.0))
            (`GameplayStatics.PlaySound2D` "/Game/Unlockables/Pop.Pop" 25.0 1.0 0.0 null null))
          (set `/Game/Data/SaveData_PlayerInfo.GameEnded` false _output_get)
          (`GameplayStatics.SaveGameToSlot` _output_get "MasterSave"))))))

(event `Key|G`
  (params (Key :type "Key Structure"))
  ;[1 1 1] Meant for testing
)

(event `Key|F`
  (params (Key :type "Key Structure"))
  ;[1 1 1] Meant for testing
)

(fn `UserConstructionScript`)