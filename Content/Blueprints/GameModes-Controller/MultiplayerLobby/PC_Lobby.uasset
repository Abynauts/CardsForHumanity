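; Player controller for the multiplayer lobby, handling host and client UI, deck sharing and player numbers.
; BeginPlay branches on authority to create the matching lobby widget and blend saved decks into GS_Lobby, with clients also sending theirs to the server.
; Events relay player numbers, player lists and deck checkbox changes, retrying until the client widget exists.
; DataValidation stores the lobby name or exits to the main menu; click-to-kick is unfinished.
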(event `DataValidation`
  (if (`self.GotLobbyName`)
    (`KismetSystemLibrary.K2_ClearAndInvalidateTimerHandle` (`self.PlayerJoined_Timer`))
    (`self.RemovedFromLobby`)
    (else
      (bind _asgs_lobby (cast `/Game/Blueprints/GameModes-Controller/MultiplayerLobby/GS_Lobby` (`GameplayStatics.GetGameState`)))
      (set `/Game/Blueprints/GameModes-Controller/Steam_GameInstance.PotentialJoinedMatch` (`/Game/Blueprints/GameModes-Controller/MultiplayerLobby/GS_Lobby.LobbyName` _asgs_lobby) (`self.As Steam Game Instance`))
      (set `self.GotLobbyName` true))))

(event `RemovedFromLobby`
  (set `/Game/Blueprints/GameModes-Controller/Steam_GameInstance.LobbyWasFull` true (cast `/Game/Blueprints/GameModes-Controller/Steam_GameInstance` (`GameplayStatics.GetGameInstance`) :!pure true))
  (`GameplayStatics.OpenLevelBySoftObjectPtr` "/Game/Maps/Map_MainMenu.Map_MainMenu")
  (`DestroySessionCallbackProxy.DestroySession` self))

(event `self.ReceiveBeginPlay`
  (bind _asgs_lobby (cast `/Game/Blueprints/GameModes-Controller/MultiplayerLobby/GS_Lobby` (`GameplayStatics.GetGameState`)))
  (set `self.As GS Lobby` _asgs_lobby)
  (bind _assteam_game_instance (cast `/Game/Blueprints/GameModes-Controller/Steam_GameInstance` (`GameplayStatics.GetGameInstance`)))
  (set `self.As Steam Game Instance` _assteam_game_instance)
  (bind _aslobby_character (cast `/Game/Blueprints/GameModes-Controller/MultiplayerLobby/LobbyCharacter` (`GameplayStatics.GetPlayerPawn` 0)))
  (set `self.Lobby Character` _aslobby_character)
  (if (`self.IsLocalController`)
    (`/Engine/EditorBlueprintResources/ActorMacros.Switch Has Authority`
      (:`Authority`
        (`self.SR_SendDecks`)
        (set `self.HasAuthority?` true)
        (`|CreateWidget` "/Game/Blueprints/GameModes-Controller/MultiplayerLobby/Widget_LobbyHostScreen.Widget_LobbyHostScreen_C"))
      (:`Remote`
        (`self.CL_SendDecks`)
        (set `self.HasAuthority?` false)
        (bind _returnvalue (`|CreateWidget` "/Game/Blueprints/GameModes-Controller/MultiplayerLobby/Widget_LobbyClientScreen.Widget_LobbyClientScreen_C"))
        (bind _output_get (set `self.ClientWidget` _returnvalue))
        (`UserWidget.AddToViewport` _output_get 0)))))

(event `CL_SendDecks`
  ;[0.5019 1 0.3674] Code revolving around deck info collection
  (bind _as_save_data_player_info (`/Game/Data/Libraries/BPFL_DeckOps.DeckCast`))
  (bind _asgs_lobby (cast `/Game/Blueprints/GameModes-Controller/MultiplayerLobby/GS_Lobby` (`GameplayStatics.GetGameState`)))
  (bind _decks (`/Game/Data/SaveData_PlayerInfo.Decks` _as_save_data_player_info))
  (`/Game/Blueprints/GameModes-Controller/MultiplayerLobby/GS_Lobby.DeckBlend` _asgs_lobby _decks)
  (`self.SR_ClientSend` _asgs_lobby _decks))

(event `SR_SetPlayerNumber_Lobby`
  (params (Num :type Integer))
  ;[1 0.4184 0.4184] Set's a player number everytime someone joins
  (bind _output_get (set `self.PlayerNumberLobby` Num))
  (`self.CL_SetPlayerNumber_Lobby` _output_get))

(event `SR_ClientSend`
  (params (Target :type "/Game/Blueprints/GameModes-Controller/MultiplayerLobby/GS_Lobby Object Reference") (TargetArray :type "Array of /Game/Data/S_Deck Structure (by ref)"))
  ;[0.5019 1 0.3674] Code revolving around deck info collection
  (`/Game/Blueprints/GameModes-Controller/MultiplayerLobby/GS_Lobby.DeckBlend` Target TargetArray))

(event `CL_SetPlayerNumber_Lobby`
  (params (Num :type Integer))
  ;[1 0.4184 0.4184] Set's a player number everytime someone joins
  (bind _output_get (set `self.PlayerNumberLobby` Num))
  (`self.MC_SetPlayerNumber_Lobby` _output_get))

(event `MC_SetPlayerNumber_Lobby`
  (params (Num :type Integer))
  ;[1 0.4184 0.4184] Set's a player number everytime someone joins
  (set `self.PlayerNumberLobby` Num))

(event `SR_SendDecks`
  ;[0.5019 1 0.3674] Code revolving around deck info collection
  (bind _as_save_data_player_info (`/Game/Data/Libraries/BPFL_DeckOps.DeckCast`))
  (bind _asgs_lobby (cast `/Game/Blueprints/GameModes-Controller/MultiplayerLobby/GS_Lobby` (`GameplayStatics.GetGameState`)))
  (`/Game/Blueprints/GameModes-Controller/MultiplayerLobby/GS_Lobby.DeckBlend` _asgs_lobby (`/Game/Data/SaveData_PlayerInfo.Decks` _as_save_data_player_info)))

(event `CreateMenus`
  ;[0.7031 0.4481 0] UI Manipulation
  (if (`self.IsLocalPlayerController`)
    (`/Engine/EditorBlueprintResources/ActorMacros.Switch Has Authority`
      (:`Authority`
        (if (not (`self.StopFromDuplicating`))
          (bind _returnvalue (`|CreateWidget` "/Game/Blueprints/GameModes-Controller/MultiplayerLobby/Widget_LobbyHostScreen.Widget_LobbyHostScreen_C"))
          (bind _output_get (set `self.LobbyWidget` _returnvalue))
          (`UserWidget.AddToViewport` _output_get 0)
          (set `self.StopFromDuplicating` true)))
      (:`Remote`
        (set `self.LobbyWidget` (`self.ClientWidget`))))))

(event `UpdateCheckbox`
  (params (CheckboxStatus :type Boolean) (CheckArrayIndex :type Integer))
  ;[0.7031 0.4481 0] UI Manipulation
  (bind _aswidget_lobby_client_screen (cast `/Game/Blueprints/GameModes-Controller/MultiplayerLobby/Widget_LobbyClientScreen` (`self.LobbyWidget`)))
  (`/Game/Blueprints/GameModes-Controller/MultiplayerLobby/Widget_LobbyClientScreen.CheckUpdate` _aswidget_lobby_client_screen CheckboxStatus CheckArrayIndex))

(event `UpdatePlayerList`
  (params (PlayerInfo :type "Array of /Game/Networking/Widgets/PlayerInfoStuct Structure"))
  (bind _lobbywidget (`self.LobbyWidget`))
  ;[0.7031 0.4481 0] UI Manipulation
  (set `self.Connected Player Info` PlayerInfo)
  (`/Engine/EditorBlueprintResources/ActorMacros.Switch Has Authority`
    (:`Authority`
      (bind _aswidget_lobby_host_screen (cast `/Game/Blueprints/GameModes-Controller/MultiplayerLobby/Widget_LobbyHostScreen` _lobbywidget))
      (`/Game/Blueprints/GameModes-Controller/MultiplayerLobby/Widget_LobbyHostScreen.UpdatePlayerList` _aswidget_lobby_host_screen (`self.Connected Player Info`)))
    (:`Remote`
      (`/Engine/EditorBlueprintResources/StandardMacros.IsValid` _lobbywidget :!label _label
        (:`Is Valid`
          (bind _aswidget_lobby_client_screen (cast `/Game/Blueprints/GameModes-Controller/MultiplayerLobby/Widget_LobbyClientScreen` _lobbywidget))
          (`/Game/Blueprints/GameModes-Controller/MultiplayerLobby/Widget_LobbyClientScreen.UpdatePlayerList` _aswidget_lobby_client_screen (`self.Connected Player Info`)))
        (:`Is Not Valid`
          (`KismetSystemLibrary.Delay` 0.2)
          (goto _label))))))

(event `Key|LeftMouseButton`
  (params (Key :type "Key Structure"))
  ;[1 1 1] Potential code for kicking players
  (:`Pressed`
    (`/Engine/EditorBlueprintResources/ActorMacros.Switch Has Authority`
      (:`Authority`
        (if (`.ReturnValue` (`self.GetHitResultUnderCursorForObjects` (`GameplayStatics.GetPlayerController` 0) (`|MakeArray` "ObjectTypeQuery3" :!type "EObjectTypeQuery Enum") true))
          _)))))

(fn `CL_SetPlayerNumber`
  (params (Num1 :type Integer)))

(fn `UserConstructionScript`)