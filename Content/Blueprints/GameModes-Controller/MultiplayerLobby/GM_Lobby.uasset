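; Game mode for the Steam multiplayer lobby, managing player joins, departures, spawn spots and displayed names.
; PostLogin registers each PC_Lobby, builds the shared player list and pushes it to every controller's menus; over-capacity joins get a kick timer.
; Names come from the MasterSave slot, falling back to Steam names.
; ChoosePlayerStart assigns indexed PlayerStarts; logout rebuilds the list and repositions lobby characters in a row.
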(event `Show Player Names`
  (bind _allpcs (`self.AllPCs`))
  (bind _as_save_data_player_info (`self.As Save Data Player Info`))
  (bind _nichardname (`/Game/Data/SaveData_PlayerInfo.NichardName` _as_save_data_player_info))
  ;[1 1 1] Sean's Testing Code: Currently, names (Nichard names and Steam names) appear properly on host at least in the editor
  (`KismetSystemLibrary.Delay` 5.0) ; Might need to become a data validation
  (for (_ _array_index) _allpcs
    (bind _returnvalue (`GameplayStatics.LoadGameFromSlot` "MasterSave" _array_index))
    (bind _assave_data_player_info (cast `/Game/Data/SaveData_PlayerInfo` _returnvalue))
    (set `self.As Save Data Player Info` _assave_data_player_info)
    (bind _aslobby_character (cast `/Game/Blueprints/GameModes-Controller/MultiplayerLobby/LobbyCharacter` (`GameplayStatics.GetPlayerCharacter` (`KismetArrayLibrary.Array_LastIndex` _allpcs))))
    (if (`/Game/Data/SaveData_PlayerInfo.IsUsingSteamName` _as_save_data_player_info)
      (bind _playername_text (`/Game/Blueprints/GameModes-Controller/MultiplayerLobby/Widget_PlayerName.PlayerName_Text` (`/Game/Blueprints/GameModes-Controller/MultiplayerLobby/LobbyCharacter.Player Card` _aslobby_character)))
      (`TextBlock.SetText` _playername_text (`KismetTextLibrary.Conv_StringToText` (`AdvancedSessionsLibrary.GetPlayerName` (`self.As PC Lobby`))) :!label _label)
      (elif (`KismetTextLibrary.EqualEqual_TextText` _nichardname "")
        (goto _label)
        (else
          (`TextBlock.SetText` _playername_text _nichardname))))))

(event `self.K2_PostLogin`
  (params (NewPlayer :type "PlayerController Object Reference"))
  ;[0 0 0] Player Connection/Disconnection
  ;;[1 1 1] Player Connect Events
  ;;;[0.3714 1 0.9901] Makes sure player can't join a full lobby. If they do, they are kicked from the game immediately.
  (if (< (`KismetArrayLibrary.Array_Length` (`self.ConnectedPlayerInfo`)) (`/Game/Blueprints/GameModes-Controller/Steam_GameInstance.Max Number Of Players Per Session` (cast `/Game/Blueprints/GameModes-Controller/Steam_GameInstance` (`GameplayStatics.GetGameInstance`) :!pure true)))
    (`PlayerController.SetViewTargetWithBlend` NewPlayer (`self.LevelCam`) 0.0 "VTBlend_Linear" 0.0 false)
    (bind _aspc_lobby (cast `/Game/Blueprints/GameModes-Controller/MultiplayerLobby/PC_Lobby` NewPlayer))
    (bind _output_get (set `self.As PC Lobby` _aspc_lobby))
    (bind _returnvalue (`KismetArrayLibrary.Array_Add` (`self.AllPCs`) _output_get))
    (bind _output_get_2 (set `/Game/Blueprints/GameModes-Controller/MultiplayerLobby/PC_Lobby.PlayerNumberLobby` _returnvalue _output_get))
    (`/Game/Blueprints/GameModes-Controller/MultiplayerLobby/PC_Lobby.SR_SetPlayerNumber_Lobby` _output_get _output_get_2)
    (set `self.PlayerSpawnIndex` (+ (`self.PlayerSpawnIndex`) 1))
    (`self.Show Player Names`)
    ;;;[1 0 0] This is the menu stuff. I will be able to get rid of a lot of this later. I keep it connected right now as a check to make sure the card names match.
    (bind _returnvalue_2 (`GameplayStatics.LoadGameFromSlot` "MasterSave"))
    (bind _assave_data_player_info (cast `/Game/Data/SaveData_PlayerInfo` _returnvalue_2))
    (if (`/Game/Data/SaveData_PlayerInfo.IsUsingSteamName` _assave_data_player_info)
      (bind _output_get_3 (set `/Game/Blueprints/GameModes-Controller/MultiplayerLobby/PC_Lobby.PlayerInfo` (make `/Game/Networking/Widgets/PlayerInfoStuct` (`KismetTextLibrary.Conv_StringToText` (`AdvancedSessionsLibrary.GetPlayerName` (`self.As PC Lobby`)))) (`self.As PC Lobby`) :!label _label_2))
      (`KismetArrayLibrary.Array_Add` (`self.ConnectedPlayerInfo`) _output_get_3)
      (else
        (bind _nichardname (`/Game/Data/SaveData_PlayerInfo.NichardName` _assave_data_player_info))
        (if (`KismetTextLibrary.EqualEqual_TextText` _nichardname "")
          (goto _label_2)
          (else
            (bind _output_get_4 (set `/Game/Blueprints/GameModes-Controller/MultiplayerLobby/PC_Lobby.PlayerInfo` (make `/Game/Networking/Widgets/PlayerInfoStuct` _nichardname) (`self.As PC Lobby`)))
            (`KismetArrayLibrary.Array_Add` (`self.ConnectedPlayerInfo`) _output_get_4)))))
    (`KismetSystemLibrary.Delay` 1.0)
    (for _array_element (`self.AllPCs`)
      (`/Game/Blueprints/GameModes-Controller/MultiplayerLobby/PC_Lobby.CreateMenus` _array_element)
      (`/Game/Blueprints/GameModes-Controller/MultiplayerLobby/PC_Lobby.UpdatePlayerList` _array_element (`self.ConnectedPlayerInfo`)))
    (else
      (bind _aspc_lobby_2 (cast `/Game/Blueprints/GameModes-Controller/MultiplayerLobby/PC_Lobby` NewPlayer))
      (bind _returnvalue_3 (`KismetSystemLibrary.K2_SetTimerDelegate` (`|CreateDelegate` _aspc_lobby_2 :!event `DataValidation`) 0.01 true))
      (set `/Game/Blueprints/GameModes-Controller/MultiplayerLobby/PC_Lobby.PlayerJoined_Timer` _returnvalue_3 _aspc_lobby_2))))

(event `self.K2_OnSwapPlayerControllers`
  (params (OldPC :type "PlayerController Object Reference") (NewPC :type "PlayerController Object Reference"))
  ;[0 0 0] Player Connection/Disconnection
  ;;[1 1 1] Player Connect Events
  (bind _aspc_lobby (cast `/Game/Blueprints/GameModes-Controller/MultiplayerLobby/PC_Lobby` NewPC))
  (`KismetArrayLibrary.Array_Add` (`self.AllPCs`) _aspc_lobby))

(event `BeenKicked`
  (params (`Player ID` :type Integer))
  ;[0 0 0] Player Connection/Disconnection
  (`/Game/Blueprints/GameModes-Controller/MultiplayerLobby/PC_Lobby.KickedFromLobby` (`|GetArrayItem` (`self.AllPCs`) `Player ID`)))

(event `self.K2_OnLogout`
  (params (ExitingController :type "Controller Object Reference"))
  ;[0 0 0] Player Connection/Disconnection
  ;;[1 1 1] Disconnect Event
  (if (not (`self.SessionDestroyed`))
    (bind _aspc_lobby (cast `/Game/Blueprints/GameModes-Controller/MultiplayerLobby/PC_Lobby` ExitingController))
    (`KismetArrayLibrary.Array_RemoveItem` (`self.AllPCs`) _aspc_lobby)
    (`self.UpdatePlayerListsWhenPlayerLeaves`)
    (if (< (`KismetArrayLibrary.Array_Length` (`self.ConnectedPlayerInfo`)) (`/Game/Blueprints/GameModes-Controller/Steam_GameInstance.Max Number Of Players Per Session` (cast `/Game/Blueprints/GameModes-Controller/Steam_GameInstance` (`GameplayStatics.GetGameInstance`) :!pure true)))
      (`self.UpdatePlayerPositions`))))

(event `UpdatePlayerPositions`
  (set `self.PlayerSpawnIndex` (- (`self.PlayerSpawnIndex`) 1))
  (for (_ _array_index) (`self.PlayerStarts`)
    (bind _aslobby_character (cast `/Game/Blueprints/GameModes-Controller/MultiplayerLobby/LobbyCharacter` (`GameplayStatics.GetPlayerCharacter` _array_index)))
    (`SceneComponent.K2_SetWorldLocation` (`Character.CapsuleComponent` _aslobby_character) (`KismetMathLibrary.MakeVector` 350.0 (`self.SpawnLocation`) -300.0) false false)
    (set `self.SpawnLocation` (+ (`self.SpawnLocation`) 100.0)))
  (set `self.SpawnLocation` -200.0))

(event `UpdatePlayerListsWhenPlayerLeaves`
  (`KismetArrayLibrary.Array_Clear` (`self.ConnectedPlayerInfo`))
  (bind _returnvalue (`GameplayStatics.LoadGameFromSlot` "MasterSave"))
  (bind _assave_data_player_info (cast `/Game/Data/SaveData_PlayerInfo` _returnvalue))
  (if (`/Game/Data/SaveData_PlayerInfo.IsUsingSteamName` _assave_data_player_info)
    (for _array_element (`self.AllPCs`) :!label _label_3
      (set `self.UpdatePlayerList Array Element` _array_element)
      (bind _output_get (set `/Game/Blueprints/GameModes-Controller/MultiplayerLobby/PC_Lobby.PlayerInfo` (make `/Game/Networking/Widgets/PlayerInfoStuct` (`KismetTextLibrary.Conv_StringToText` (`AdvancedSessionsLibrary.GetPlayerName` (`self.UpdatePlayerList Array Element`)))) (`self.UpdatePlayerList Array Element`)))
      (`KismetArrayLibrary.Array_Add` (`self.ConnectedPlayerInfo`) _output_get))
    (else
      (bind _nichardname (`/Game/Data/SaveData_PlayerInfo.NichardName` _assave_data_player_info))
      (if (`KismetTextLibrary.EqualEqual_TextText` _nichardname "")
        (goto _label_3)
        (else
          (for _array_element_2 (`self.AllPCs`)
            (set `self.UpdatePlayerList Array Element` _array_element_2)
            (bind _output_get_2 (set `/Game/Blueprints/GameModes-Controller/MultiplayerLobby/PC_Lobby.PlayerInfo` (make `/Game/Networking/Widgets/PlayerInfoStuct` _nichardname) (`self.UpdatePlayerList Array Element`)))
            (`KismetArrayLibrary.Array_Add` (`self.ConnectedPlayerInfo`) _output_get_2))))))
  (`KismetSystemLibrary.Delay` 1.0)
  (for _array_element_3 (`self.AllPCs`)
    (`/Game/Blueprints/GameModes-Controller/MultiplayerLobby/PC_Lobby.UpdatePlayerList` _array_element_3 (`self.ConnectedPlayerInfo`))))

(fn `ChoosePlayerStart`
  (params (Player :type "Controller Object Reference"))
  (returns (ReturnValue :type "Actor Object Reference"))
  (if (< (`KismetArrayLibrary.Array_Length` (`self.ConnectedPlayerInfo`)) (`/Game/Blueprints/GameModes-Controller/Steam_GameInstance.Max Number Of Players Per Session` (cast `/Game/Blueprints/GameModes-Controller/Steam_GameInstance` (`GameplayStatics.GetGameInstance`) :!pure true)))
    (set `self.SelectedPlayerStart` (`|GetArrayItem` (`self.PlayerStarts`) (`self.PlayerSpawnIndex`)))
    (return (`self.SelectedPlayerStart`))))

(fn `UserConstructionScript`
  (bind _outactors (`GameplayStatics.GetAllActorsOfClass` "/Script/Engine.PlayerStart"))
  (set `self.PlayerStarts` _outactors))