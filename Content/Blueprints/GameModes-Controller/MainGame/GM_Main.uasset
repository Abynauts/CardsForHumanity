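; Main game mode for a multiplayer card game with a rotating Card Reader, driving rounds through GS_Main and each PC_Main.
; BeginPlay registers and numbers controllers, then a looping timer gates start on player count, valid PlayerStates and possessed camera pawns before copying GameInstance modifiers.
; Events advance phases, black cards and readers, shuffling non-readers and supporting ReaderPick and random DoBetter rounds.
; Any logout ends the session for everyone, returning to the main menu.
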(event `self.K2_PostLogin`
  (params (NewPlayer :type "PlayerController Object Reference"))
  ;[0 0 0] NOTE: Start here—login events don't trigger since there's no reconnection
)

(event `IncrementBlackCard`
  (bind _asgs_main (cast `/Game/Blueprints/GameModes-Controller/MainGame/GS_Main` (`GameplayStatics.GetGameState`)))
  (for _array_element (`self.AllPCs`)
    (bind _blackcard (`/Game/Blueprints/GameModes-Controller/MainGame/GS_Main.BlackCard` _asgs_main))
    (`/Game/Blueprints/GameModes-Controller/MainGame/PC_Main.BlackCardDisplay` _array_element (break `/Game/Data/S_BlackCard` (`.BlackCard_5_B6091C064EE4709FD05967B9850E05F8` (break `/Game/Data/S_BlackDetailed` _blackcard))) (`.Answers_25_19CBC36D47CEFB152C5F56AD7D7C5232` (break `/Game/Data/S_BlackCard` (`.BlackCard_5_B6091C064EE4709FD05967B9850E05F8` (break `/Game/Data/S_BlackDetailed` _blackcard))))))
  (`/Engine/EditorBlueprintResources/StandardMacros.IncrementInt` (`self.BlackCardIndex`)))

(event `self.ReceiveBeginPlay`
  (`self.GetPlayerSpawnInfo`)
  (`KismetSystemLibrary.Delay` 1.5)
  (bind _outactors (`GameplayStatics.GetAllActorsOfClass` "/Game/Blueprints/GameModes-Controller/MainGame/PC_Main.PC_Main_C"))
  (for _array_element _outactors
    (if (`Controller.IsLocalPlayerController` _array_element)
      _
      (else
        _))
    (bind _returnvalue (`KismetArrayLibrary.Array_Add` (`self.AllPCs`) _array_element))
    (bind _output_get (set `/Game/Blueprints/GameModes-Controller/MainGame/PC_Main.PlayerNumber` _returnvalue _array_element))
    (`/Game/Blueprints/GameModes-Controller/MainGame/PC_Main.SR_SetPlayerNumber` _array_element _output_get))
  (set `self.PlayerCount` (`KismetArrayLibrary.Array_Length` (`self.AllPCs`)))
  (if (not (`KismetSystemLibrary.K2_IsTimerActiveHandle` (`self.BeginPlay_Timer`)))
    (bind _returnvalue_2 (`KismetSystemLibrary.K2_SetTimerDelegate` (`|CreateDelegate` :!event `BeginPlay_Validation`) 0.1 true))
    (set `self.BeginPlay_Timer` _returnvalue_2)))

(event `BeginPlay_Validation`
  (bind _assteam_game_instance (cast `/Game/Blueprints/GameModes-Controller/Steam_GameInstance` (`GameplayStatics.GetGameInstance`))
    (:`then`
      _)
    (:`CastFailed`
      _))
  (if (== (`/Game/Blueprints/GameModes-Controller/Steam_GameInstance.StartingPlayerCount` _assteam_game_instance) (`self.PlayerCount`))
    (`KismetSystemLibrary.K2_ClearAndInvalidateTimerHandle` (`self.BeginPlay_Timer`))
    (for _array_element (`self.AllPCs`) :!label _label
      (`/Engine/EditorBlueprintResources/StandardMacros.IsValid` (`Controller.PlayerState` _array_element)
        (:`Is Not Valid`
          (goto _label))))
    (set `self.AllPlayersValid?` true)
    (for _array_element_2 (`self.AllPCs`) :!label _label_2
      (if (not (`/Game/Blueprints/GameModes-Controller/MainGame/PC_Main.PawnPossessed?` _array_element_2))
        (`KismetSystemLibrary.Delay` 0.2)
        (goto _label_2)))
    (set `self.AllPawnsPossessed?` true)
    (bind _asgs_main (cast `/Game/Blueprints/GameModes-Controller/MainGame/GS_Main` (`GameplayStatics.GetGameState`)))
    (`/Game/Blueprints/GameModes-Controller/MainGame/GS_Main.CL_GM_ValidationComplete` _asgs_main)
    (`self.GM_ModSet` _assteam_game_instance)))

(event `GM_ModSet`
  (params (GameInstance :type "/Game/Blueprints/GameModes-Controller/Steam_GameInstance Object Reference"))
  ;[1 1 1] Modifier Set
  (`|ExecutionSequence`
    (:`then_0`
      (set `self.Mod_Redo_GM` (`/Game/Blueprints/GameModes-Controller/Steam_GameInstance.Mod_Redo` GameInstance)))
    (:`then_1`
      (set `self.Mod_Improv_GM` (`/Game/Blueprints/GameModes-Controller/Steam_GameInstance.Mod_Improv` GameInstance)))
    (:`then_2`
      (set `self.Mod_TradeIn_GM` (`/Game/Blueprints/GameModes-Controller/Steam_GameInstance.Mod_TradeIn` GameInstance)))
    (:`then_3`
      (set `self.Mod_Switcheroo_GM` (`/Game/Blueprints/GameModes-Controller/Steam_GameInstance.Mod_Switcheroo` GameInstance)))
    (:`then_4`
      (set `self.Mod_ReaderPick_GM` (`/Game/Blueprints/GameModes-Controller/Steam_GameInstance.Mod_ReaderPick` GameInstance)))
    (:`then_5`
      (set `self.Mod_DoBetter_GM` (`/Game/Blueprints/GameModes-Controller/Steam_GameInstance.Mod_DoBetter` GameInstance)))))

(event `ChooseCzar`
  ;[1 1 1] Sets the first Card Reader
  (`/Game/Blueprints/GameModes-Controller/MainGame/PC_Main.CardCzar` (`|GetArrayItem` (`self.AllPCs`)) false) ; Set the host as the first reader
  (set `self.CzarIndex` 0)
  (for _array_element (`self.AllPCs`)
    (if (not (`/Game/Blueprints/GameModes-Controller/MainGame/PC_Main.CardCzar?` _array_element))
      (`KismetArrayLibrary.Array_Add` (`self.ArrangementShuffler`) _array_element) ; Non-readers added to \nan array
    ))
  (`KismetArrayLibrary.Array_Shuffle` (`self.ArrangementShuffler`))
  (if (`self.Mod_ReaderPick_GM`)
    (set `self.ReaderPickActive?` true) ; Activate picking the reader for\nthe ReaderPick modifier
  )
  (if (== (`self.CzarIndex`) (- (`self.PlayerCount`) 1))
    (set `self.CzarIndex` 0) ; Resets reader order if \nall players have had a chance\nto be reader
    (else
      (`/Engine/EditorBlueprintResources/StandardMacros.IncrementInt` (`self.CzarIndex`)))))

(event `Phase1Increment`
  (bind _playersfinished (`self.PlayersFinished`))
  (`/Engine/EditorBlueprintResources/StandardMacros.IncrementInt` _playersfinished
    (:`  `
      (if (== _playersfinished (- (`self.PlayerCount`) 1))
        (`KismetSystemLibrary.Delay` 1.5)
        (bind _asgs_main (cast `/Game/Blueprints/GameModes-Controller/MainGame/GS_Main` (`GameplayStatics.GetGameState`)))
        (`/Game/Blueprints/GameModes-Controller/MainGame/GS_Main.CL_Phase2Prep` _asgs_main)))))

(event `EnableSelection`
  (for _array_element (`self.AllPCs`)
    (if (`/Game/Blueprints/GameModes-Controller/MainGame/PC_Main.CardCzar?` _array_element)
      (`/Game/Blueprints/GameModes-Controller/MainGame/PC_Main.CL_EnableSelection` _array_element))))

(event `Phase3Prep`
  (bind _asgs_main (cast `/Game/Blueprints/GameModes-Controller/MainGame/GS_Main` (`GameplayStatics.GetGameState`)))
  (`/Game/Blueprints/GameModes-Controller/MainGame/GS_Main.CL_Phase3Prep` _asgs_main))

(event `GM_VariableFlush`
  (set `self.PlayersFinished` 0)
  (`KismetArrayLibrary.Array_Clear` (`self.ArrangementShuffler`))
  (for _array_element (`self.AllPCs`)
    (`/Game/Blueprints/GameModes-Controller/MainGame/PC_Main.PC_VariableFlush` _array_element)))

(event `self.K2_OnLogout`
  (params (ExitingController :type "Controller Object Reference"))
  ;[1 1 1] Kicks all players from game when someone leaves.
  (for _array_element (`self.AllPCs`)
    (`/Engine/EditorBlueprintResources/StandardMacros.IsValid` _array_element
      (:`Is Valid`
        (`/Game/Blueprints/GameModes-Controller/MainGame/PC_Main.PlayerLeftMainGame` _array_element)
        (`DestroySessionCallbackProxy.DestroySession` _array_element
          (:`OnSuccess`
            (`GameplayStatics.OpenLevelBySoftObjectPtr` "/Game/Maps/Map_MainMenu.Map_MainMenu")))))))

(event `IncrementCzar`
  (bind _output (`|GetArrayItem` (`self.AllPCs`) (`self.ReaderPick_Index`)))
  (bind _output_2 (`|GetArrayItem` (`self.AllPCs`) (`self.CzarIndex`)))
  ;[1 1 1] Sets the next Reader
  (if (`self.Mod_DoBetter_GM`)
    (bind _dobetterround_ (`self.DoBetterRandomizer`))
    (bind _asgs_main (cast `/Game/Blueprints/GameModes-Controller/MainGame/GS_Main` (`GameplayStatics.GetGameState`)))
    (bind _output_get (set `/Game/Blueprints/GameModes-Controller/MainGame/GS_Main.DoBetterRound?_GS` _dobetterround_ _asgs_main))
    (bind _output_get_2 (set `self.Do Better Round?` _output_get))
    (if (`self.ReaderPickActive?`)
      (`/Game/Blueprints/GameModes-Controller/MainGame/PC_Main.CardCzar` _output _output_get_2)
      (else
        (`/Game/Blueprints/GameModes-Controller/MainGame/PC_Main.CardCzar` _output_2 _output_get_2)))
    (elif (`self.ReaderPickActive?`)
      (`/Game/Blueprints/GameModes-Controller/MainGame/PC_Main.CardCzar` _output false)
      (else
        (`/Game/Blueprints/GameModes-Controller/MainGame/PC_Main.CardCzar` _output_2 false))))
  (for _array_element (`self.AllPCs`)
    (if (not (`/Game/Blueprints/GameModes-Controller/MainGame/PC_Main.CardCzar?` _array_element))
      (`KismetArrayLibrary.Array_Add` (`self.ArrangementShuffler`) _array_element)))
  (`KismetArrayLibrary.Array_Shuffle` (`self.ArrangementShuffler`))
  (if (== (`self.CzarIndex`) (- (`self.PlayerCount`) 1))
    (set `self.CzarIndex` 0)
    (else
      (`/Engine/EditorBlueprintResources/StandardMacros.IncrementInt` (`self.CzarIndex`)))))

(event `GM_ReaderPick_SetNextReader`
  (params (PC_NextReader :type "/Game/Blueprints/GameModes-Controller/MainGame/PC_Main Object Reference") (NewParam :type Integer))
  ;[1 1 1] Sets the next Reader
  (set `self.ReaderPick_Index` NewParam))

(event `Endgame`
  (for _array_element (`self.AllPCs`)
    (`/Game/Blueprints/GameModes-Controller/MainGame/PC_Main.EndSequence` _array_element)))

(fn `DoBetterRandomizer`
  (returns (`DoBetterRound?` :type Boolean))
  (bind _returnvalue (and (<= (`KismetMathLibrary.RandomIntegerInRange` 0 40) (`self.DoBetter_Chance`)) (`self.DoBetter_GracePeriodOver?`)))
  (if _returnvalue
    (set `self.DoBetter_GracePeriodOver?` false)
    (else
      (set `self.DoBetter_GracePeriodOver?` true)))
  (return _returnvalue))

(fn `GetPlayerSpawnInfo`
  (bind _outactors (`GameplayStatics.GetAllActorsOfClass` "/Script/Engine.PlayerStart"))
  (for _array_element _outactors
    (`KismetArrayLibrary.Array_Add` (`self.SpawnInfo`) (make `/Game/Data/S_SpawnInfo` _array_element (`self.GetTransform` _array_element))))
  (return))

(fn `Player Spawn`
  (params (`New Player` :type "/Game/Blueprints/GameModes-Controller/MainGame/PC_Main Object Reference") (SequenceIndex :type Integer))
  (returns (NewSequenceIndex :type Integer))
  (bind _returnvalue (`Controller.K2_GetPawn` `New Player`))
  (bind (_output_playerstart _output_spawntransform) (break `/Game/Data/S_SpawnInfo` (`|GetArrayItem` (`self.SpawnInfo`) (`|GetArrayItem` (`self.SpawnSequence`) SequenceIndex))))
  ;[0 0 0] Phase 0: Spawn players, deal initial hand, choose a card czar
  (`/Engine/EditorBlueprintResources/StandardMacros.IsValid` _returnvalue ; Determines if the player already controls\nan actor. If so, destroys the actor, spawns\na new one.
    (:`Is Valid`
      (`self.K2_DestroyActor` _returnvalue))
    (:`Is Not Valid`
      _))
  (bind _returnvalue_2 (`|SpawnActorFromClass` "/Game/Blueprints/GameModes-Controller/MainGame/Pawn_MainGameCamera.Pawn_MainGameCamera_C" _output_spawntransform "Undefined" "OverrideRootScale" null null))
  (`/Game/Blueprints/GameModes-Controller/MainGame/Pawn_MainGameCamera.DealHand_Validation` _returnvalue_2)
  (`Controller.Possess` `New Player` _returnvalue_2)
  (set `/Game/Blueprints/GameModes-Controller/MainGame/PC_Main.ControlledPawn` _returnvalue_2 `New Player`)
  (set `/Game/Blueprints/GameModes-Controller/MainGame/PC_Main.PawnPossessed?` true `New Player`)
  (bind _result (`/Engine/EditorBlueprintResources/StandardMacros.IncrementInt` (`self.Sequence Index`))
    (:`  `
      (return _result))))

(fn `UserConstructionScript`)