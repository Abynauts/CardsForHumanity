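; Player controller for the online card game's main match, handling each player's reader role, card limits, selection phase and end-of-game results.
; It creates local HUD and modifier widgets, using delay-retry loops to wait for pawn, hand or widgets.
; SR/CL/MC events relay player number, selection and round resets between GM_Main, clients and pawn.
; EndSequence saves wins and XP, writes achievements and shows the victory or loser screen.
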(event `PlayerLeftMainGame`
  (set `/Game/Blueprints/GameModes-Controller/Steam_GameInstance.PlayerLeftGame` true (cast `/Game/Blueprints/GameModes-Controller/Steam_GameInstance` (`GameplayStatics.GetGameInstance`) :!pure true)))

(event `WHY_TF_IS_THIS_THE_ONLY_METHOD_THAT_REMOVES_EXTRA_PLAYERS`
  ;[1 1 1] Removes extra player if they somehow managed to join when a game started
  (`KismetSystemLibrary.K2_ClearAndInvalidateTimerHandle` (`self.PlayerJoined_Timer`))
  (`self.RemovePlayer`))

(event `RemovePlayer`
  ;[1 1 1] Removes extra player if they somehow managed to join when a game started
  (set `/Game/Blueprints/GameModes-Controller/Steam_GameInstance.LobbyWasFull` true (cast `/Game/Blueprints/GameModes-Controller/Steam_GameInstance` (`GameplayStatics.GetGameInstance`) :!pure true))
  (`GameplayStatics.OpenLevelBySoftObjectPtr` "/Game/Maps/Map_MainMenu.Map_MainMenu")
  (`DestroySessionCallbackProxy.DestroySession` self))

(event `self.ReceiveBeginPlay`
  ;[1 1 1] Beginplay events
  ;[1 1 1] Once we replicate "Remove All Widgets" in Widget_LobbyHostScreen, we can get rid of these nodes.
  (`WidgetLayoutLibrary.RemoveAllWidgets`)
  (`|ExecutionSequence`
    (:`then_0`
      (`KismetSystemLibrary.Delay` 0.1))
    (:`then_1`
      (`KismetSystemLibrary.Delay` 3.0)
      (bind _assteam_game_instance (cast `/Game/Blueprints/GameModes-Controller/Steam_GameInstance` (`GameplayStatics.GetGameInstance`))
        (:`then`
          (set `self.Online Game Instance` _assteam_game_instance)
          (if (`self.IsLocalPlayerController`)
            (`self.SR_SpawnPlayer`)
            (bind _returnvalue (`|CreateWidget` "/Game/Blueprints/GameModes-Controller/MainGame/Widget_ReaderDisplay.Widget_ReaderDisplay_C" self))
            (bind _output_get (set `self.ReaderWidget` _returnvalue))
            (bind _returnvalue_2 (`|CreateWidget` "/Game/Blueprints/GameModes-Controller/MainGame/Widget_ReaderDisplay_DoBetter.Widget_ReaderDisplay_DoBetter_C" self))
            (bind _output_get_2 (set `self.DoBetterWidget` _returnvalue_2))
            (`UserWidget.AddToViewport` _output_get_2 0)
            (`Widget.SetVisibility` _output_get_2 "Collapsed")
            (`UserWidget.AddToViewport` _output_get 0)
            (`Widget.SetVisibility` _output_get "Collapsed")
            (`self.ModWidgetCreate`)
            ;;[0.3036 0.7451 1] This shows the "You're the Reader" widget and turns the reader's cards gray on the first round.
            (if (`self.CardCzar?`)
              (`Widget.SetVisibility` _output_get "HitTestInvisible")
              (bind _aspawn_main_game_camera (cast `/Game/Blueprints/GameModes-Controller/MainGame/Pawn_MainGameCamera` (`GameplayStatics.GetPlayerPawn` 0)))
              (if (`/Game/Blueprints/GameModes-Controller/MainGame/Pawn_MainGameCamera.HandDealt?` _aspawn_main_game_camera) :!label _label
                (`self.TurnPlayerCardsGray`)
                (else
                  (`KismetSystemLibrary.Delay` 0.1)
                  (goto _label))))))
        (:`CastFailed`
          (`KismetSystemLibrary.PrintString` "CastFailInstance"))))))

(event `ModWidgetCreate`
  (bind _mod_improv_pc (`self.Mod_Improv_PC`))
  (bind _mod_redo_pc (`self.Mod_Redo_PC`))
  (if (or _mod_improv_pc _mod_redo_pc)
    (bind _returnvalue (`|CreateWidget` "/Game/Blueprints/GameModes-Controller/MainGame/Widget_WildCardButton.Widget_WildCardButton_C" self))
    (`UserWidget.AddToViewport` _returnvalue 0)
    (set `self.WildcardWidget` _returnvalue)
    (set `self.Mod_Improv_PC` _mod_improv_pc)
    (set `self.Mod_Redo_PC` _mod_redo_pc)))

(event `BlackCardDisplay`
  (params (BlackCardText :type Text) (AnswerCount :type Byte))
  (bind _blackcarddisplaywidget (`self.BlackCardDisplayWidget`))
  (set `self.AnswerCount` AnswerCount)
  (set `self.NextReader?` false)
  (`KismetSystemLibrary.PrintString` (`KismetStringLibrary.Conv_IntToString` (`self.PC_BlackCardIndex`)))
  (if (`self.IsLocalController`)
    (if (`self.StartupFinished?`)
      (set `/Game/Blueprints/GameModes-Controller/MainGame/Widget_BlackCardDisplay.BlackCardText` BlackCardText (`self.BlackCardDisplayWidget`))
      (else
        (`/Engine/EditorBlueprintResources/StandardMacros.IsValid` (`self.ControlledPawn`) :!label _label_2
          (:`Is Valid`
            (`/Engine/EditorBlueprintResources/StandardMacros.IsValid` _blackcarddisplaywidget
              (:`Is Valid`
                (`Widget.RemoveFromParent` _blackcarddisplaywidget))
              (:`Is Not Valid`
                _))
            (if (`/Game/Blueprints/GameModes-Controller/MainGame/Pawn_MainGameCamera.HandDealt?` (`self.ControlledPawn`)) :!label _label_3
              (set `self.StartupFinished?` true)
              (bind _returnvalue (`|CreateWidget` "/Game/Blueprints/GameModes-Controller/MainGame/Widget_BlackCardDisplay.Widget_BlackCardDisplay_C"))
              (`UserWidget.AddToViewport` _returnvalue 0)
              (set `self.BlackCardDisplayWidget` _returnvalue)
              (set `/Game/Blueprints/GameModes-Controller/MainGame/Widget_BlackCardDisplay.BlackCardText` BlackCardText _returnvalue)
              (else
                (`KismetSystemLibrary.Delay` 0.2)
                (goto _label_3))))
          (:`Is Not Valid`
            (`KismetSystemLibrary.Delay` 0.2)
            (goto _label_2)))))))

(event `SR_SpawnPlayer`
  (bind _asgm_main (cast `/Game/Blueprints/GameModes-Controller/MainGame/GM_Main` (`GameplayStatics.GetGameMode`)))
  (bind _newsequenceindex (`/Game/Blueprints/GameModes-Controller/MainGame/GM_Main.Player Spawn` _asgm_main self (`/Game/Blueprints/GameModes-Controller/MainGame/GM_Main.Sequence Index` _asgm_main)))
  (set `/Game/Blueprints/GameModes-Controller/MainGame/GM_Main.Sequence Index` _newsequenceindex _asgm_main))

(event `Improv_SubtractWildcard`
  ;[1 1 1] For Improv Game Mode
  (`/Engine/EditorBlueprintResources/StandardMacros.DecrementInt` (`self.Improv_WildCount`)))

(event `Switcheroo_Graphic`
  (if (`self.IsLocalPlayerController`)
    (bind _returnvalue (`|CreateWidget` "/Game/Blueprints/GameModes-Controller/MainGame/Widget_Switcheroo.Widget_Switcheroo_C"))
    (`UserWidget.AddToViewport` _returnvalue 0)
    (`Widget.SetVisibility` _returnvalue "Visible")
    (`KismetSystemLibrary.Delay` 3.0)
    (`Widget.RemoveFromParent` _returnvalue)))

(event `SR_SetPlayerNumber`
  (params (Num :type Integer))
  (bind _output_get (set `self.PlayerNumber` Num))
  (`self.CL_SetPlayerNumber` _output_get))

(event `Improv_WildcardWidget_Create`
  ;[1 1 1] For Improv Game Mode
  (set `/Game/Blueprints/GameModes-Controller/MainGame/Pawn_MainGameCamera.IsPaused` true (`self.ControlledPawn`))
  (set `self.Improv_CardCreatorActive?` true)
  (bind _returnvalue (`|CreateWidget` "/Game/Blueprints/CardStuff/Widget_DeckCreator_Wildcard.Widget_DeckCreator_Wildcard_C" self))
  (`UserWidget.AddToViewport` _returnvalue 0)
  (`Widget.SetVisibility` _returnvalue "Visible"))

(event `CL_SetPlayerNumber`
  (params (Num :type Integer))
  (bind _output_get (set `self.PlayerNumber` Num))
  (`self.MC_SetPlayerNumber` _output_get))

(event `CardCzar`
  (params (`DoBetterRound?` :type Boolean))
  ;[1 1 1] Sets the player as a Czar
  (if (`self.IsLocalPlayerController`)
    (set `self.CardCzar?` true)
    (if `DoBetterRound?`
      (`Widget.SetVisibility` (`self.DoBetterWidget`) "HitTestInvisible")
      (else
        (`/Engine/EditorBlueprintResources/StandardMacros.IsValid` (`self.ReaderWidget`) :!label _label_4
          (:`Is Valid`
            (`Widget.SetVisibility` (`self.ReaderWidget`) "HitTestInvisible"))
          (:`Is Not Valid`
            (`KismetSystemLibrary.Delay` 0.2)
            (goto _label_4)))))
    (set `self.IsReader?` true)
    (`self.TurnPlayerCardsGray`)
    (else
      (set `self.CardCzar?` true)
      (set `self.IsReader?` false))))

(event `Improv_WildcardWidget_Commit`
  (params (CardText :type Text) (WildcardWidget :type "/Game/Blueprints/CardStuff/Widget_DeckCreator_Wildcard Object Reference"))
  (bind _controlledpawn (`self.ControlledPawn`))
  ;[1 1 1] For Improv Game Mode
  (`/Game/Blueprints/GameModes-Controller/MainGame/Pawn_MainGameCamera.SR_Improv_SendText` _controlledpawn CardText)
  (`self.Improv_SubtractWildcard`)
  (`Widget.RemoveFromParent` WildcardWidget)
  (set `self.Improv_CardCreatorActive?` false)
  (`KismetSystemLibrary.Delay` 0.5)
  (set `/Game/Blueprints/GameModes-Controller/MainGame/Pawn_MainGameCamera.IsPaused` false _controlledpawn))

(event `MC_SetPlayerNumber`
  (params (Num :type Integer))
  (set `self.PlayerNumber` Num))

(event `Switcheroo_NewHand`
  (params (Switch_Bundle :type "Array of /Game/Data/S_WhiteDetailed Structure"))
  (`/Game/Blueprints/GameModes-Controller/MainGame/Pawn_MainGameCamera.Switcheroo_ReplaceText` (`self.ControlledPawn`) Switch_Bundle))

(event `SetIndex`
  (params (NewParam :type Integer))
  (bind _asgm_main (cast `/Game/Blueprints/GameModes-Controller/MainGame/GM_Main` (`GameplayStatics.GetGameMode`)))
  (`/Game/Blueprints/GameModes-Controller/MainGame/GM_Main.GM_ReaderPick_SetNextReader` _asgm_main null NewParam))

(event `Improv_WildcardWidget_Cancel`
  (params (`WIldcard Widget` :type "/Game/Blueprints/CardStuff/Widget_DeckCreator_Wildcard Object Reference"))
  ;[1 1 1] For Improv Game Mode
  (set `/Game/Blueprints/GameModes-Controller/MainGame/Pawn_MainGameCamera.IsPaused` false (`self.ControlledPawn`))
  (`Widget.RemoveFromParent` `WIldcard Widget`)
  (set `self.Improv_CardCreatorActive?` false))

(event `CL_EnableSelection`
  ;[1 1 1] Sets the player as a Czar
  (set `self.SelectionPhase?` true)
  (`self.TurnPlayerCardsNormalColor`)
  (`self.SR_EnableSelection`))

(event `PC_IncrementScore`
  (params (PlayerState :type "/Game/Blueprints/GameModes-Controller/MainGame/PS_Main Object Reference") (Score :type Integer))
  (`/Game/Blueprints/GameModes-Controller/MainGame/PS_Main.CL_IncrementScore` PlayerState Score))

(event `SR_EnableSelection`
  ;[1 1 1] Sets the player as a Czar
  (set `self.SelectionPhase?` true)
  (`self.TurnPlayerCardsNormalColor`))

(event `DecrementScore_PC`
  (bind _asps_main (cast `/Game/Blueprints/GameModes-Controller/MainGame/PS_Main` (`self.PlayerState`)))
  (`/Game/Blueprints/GameModes-Controller/MainGame/PS_Main.DecrementScore` _asps_main)
  (set `self.PlayerScore` (`/Game/Blueprints/GameModes-Controller/MainGame/PS_Main.PS_Score` _asps_main)))

(event `CL_CardPlayIncrement`
  ;[1 1 1] Card Incrementing
  (if (`self.IsLocalPlayerController`)
    (`/Engine/EditorBlueprintResources/StandardMacros.IncrementInt` (`self.CardsPlayed`)
      (:`  `
        (bind _asgs_main (cast `/Game/Blueprints/GameModes-Controller/MainGame/GS_Main` (`GameplayStatics.GetGameState`)))
        (if (== (`self.CardsPlayed`) (`KismetMathLibrary.Conv_ByteToInt` (`self.AnswerCount`)))
          (set `self.CardLimitReached?` true)
          (`self.SR_CardPlayIncrement`))))))

(event `SR_CardPlayIncrement`
  ;[1 1 1] Card Incrementing
  (bind _asgm_main (cast `/Game/Blueprints/GameModes-Controller/MainGame/GM_Main` (`GameplayStatics.GetGameMode`))
    (:`then`
      (`/Game/Blueprints/GameModes-Controller/MainGame/GM_Main.Phase1Increment` _asgm_main))
    (:`CastFailed`
      (`KismetSystemLibrary.PrintString` "Failed to talk with GM"))))

(event `EndSequence`
  (bind _online_game_instance (`self.Online Game Instance`))
  ;[1 1 1] Victory Sequence
  (if (`self.IsLocalController`)
    (set `self.GameEnd?` true)
    (if (`/Game/Blueprints/GameModes-Controller/MainGame/GM_Main.-GamePoints` (`self.As GM Main`))
      (bind _returnvalue (`GameplayStatics.LoadGameFromSlot` "MasterSave"))
      (bind _assave_data_player_info (cast `/Game/Data/SaveData_PlayerInfo` _returnvalue))
      (set `/Game/Data/SaveData_PlayerInfo.AmountOfWins` (+ (`/Game/Data/SaveData_PlayerInfo.AmountOfWins` _assave_data_player_info) -1) _assave_data_player_info)
      (bind _asps_main (cast `/Game/Blueprints/GameModes-Controller/MainGame/PS_Main` (`self.PlayerState`)))
      (`/Game/Data/SaveData_PlayerInfo.AddLevel&Xp` _assave_data_player_info (* (`/Game/Blueprints/GameModes-Controller/MainGame/PS_Main.PS_Score` _asps_main) -25))
      ;;[0 0 0] Anti-Achievement
      (`AchievementQueryCallbackProxy.CacheAchievements` self
        (:`OnSuccess`
          (`AchievementWriteCallbackProxy.WriteAchievementProgress` self "ACHIEVEMENT_Win50games" -2.0
            (:`then`
              _)
            (:`OnSuccess`
              _))
          ;;[1 0 0] Achievement
          (`AchievementQueryCallbackProxy.CacheAchievements` self
            (:`OnSuccess`
              (`AchievementWriteCallbackProxy.WriteAchievementProgress` self "ACHIEVEMENT_-10points" 1.0
                (:`then`
                  _)
                (:`OnSuccess`
                  _))
              (bind _returnvalue_2 (`|CreateWidget` "/Game/Blueprints/GameModes-Controller/MainGame/Widget_LoserScreen.Widget_LoserScreen_C" self))
              (`UserWidget.AddToViewport` _returnvalue_2 0)
              (set `/Game/Data/SaveData_PlayerInfo.GameEnded` true _assave_data_player_info)
              (`GameplayStatics.SaveGameToSlot` _assave_data_player_info "MasterSave")))))
      (else
        (bind _returnvalue_3 (`GameplayStatics.LoadGameFromSlot` "MasterSave"))
        (bind _assave_data_player_info_2 (cast `/Game/Data/SaveData_PlayerInfo` _returnvalue_3))
        (set `/Game/Data/SaveData_PlayerInfo.AmountOfWins` (+ (`/Game/Data/SaveData_PlayerInfo.AmountOfWins` _assave_data_player_info_2) 1) _assave_data_player_info_2)
        (bind _asps_main_2 (cast `/Game/Blueprints/GameModes-Controller/MainGame/PS_Main` (`self.PlayerState`)))
        (`/Game/Data/SaveData_PlayerInfo.AddLevel&Xp` _assave_data_player_info_2 (* (`/Game/Blueprints/GameModes-Controller/MainGame/PS_Main.PS_Score` _asps_main_2) 25))
        ;;[0.2379 1 0.4659] If you win, you get an extra 50 xp
        (if (== (`/Game/Blueprints/GameModes-Controller/MainGame/PS_Main.PS_Score` _asps_main_2) (`/Game/Blueprints/GameModes-Controller/Steam_GameInstance.FinalScore` (`self.Online Game Instance`)))
          (`/Game/Data/SaveData_PlayerInfo.AddLevel&Xp` _assave_data_player_info_2 50)
          ;;[1 0 0] Achievement
          (`AchievementQueryCallbackProxy.CacheAchievements` self
            (:`OnSuccess`
              (`AchievementWriteCallbackProxy.WriteAchievementProgress` self "ACHIEVEMENT_Win50games" 2.0
                (:`then`
                  _)
                (:`OnSuccess`
                  _))
              ;;[1 0 0] Achievement
              (if (or (`/Game/Blueprints/GameModes-Controller/Steam_GameInstance.Mod_DoBetter` _online_game_instance) (`/Game/Blueprints/GameModes-Controller/Steam_GameInstance.Mod_Improv` _online_game_instance) (`/Game/Blueprints/GameModes-Controller/Steam_GameInstance.Mod_ReaderPick` _online_game_instance) (`/Game/Blueprints/GameModes-Controller/Steam_GameInstance.Mod_Redo` _online_game_instance) (`/Game/Blueprints/GameModes-Controller/Steam_GameInstance.Mod_Switcheroo` _online_game_instance) (`/Game/Blueprints/GameModes-Controller/Steam_GameInstance.Mod_TradeIn` _online_game_instance))
                (`AchievementQueryCallbackProxy.CacheAchievements` self
                  (:`OnSuccess`
                    (`AchievementWriteCallbackProxy.WriteAchievementProgress` self "ACHIEVEMENT_ChangeItUp" 1.0
                      (:`then`
                        _)
                      (:`OnSuccess`
                        _))
                    (bind _returnvalue_4 (`|CreateWidget` "/Game/Blueprints/GameModes-Controller/MainGame/Widget_VictoryScreen.Widget_VictoryScreen_C" self :!label _label_5))
                    (`UserWidget.AddToViewport` _returnvalue_4 0)
                    (set `/Game/Data/SaveData_PlayerInfo.GameEnded` true _assave_data_player_info_2)
                    (`GameplayStatics.SaveGameToSlot` _assave_data_player_info_2 "MasterSave"))))))
          (else
            (goto _label_5)))))))

(event `PC_Phase3Prep`
  ;[1 1 1] Variable Resets
  (bind _asgm_main (cast `/Game/Blueprints/GameModes-Controller/MainGame/GM_Main` (`GameplayStatics.GetGameMode`)))
  (`/Game/Blueprints/GameModes-Controller/MainGame/GM_Main.Phase3Prep` _asgm_main))

(event `PC_VariableFlush`
  ;[1 1 1] Variable Resets
  (`/Engine/EditorBlueprintResources/ActorMacros.Switch Has Authority`
    (:`Authority`
      (`self.MC_VariableFlush`))
    (:`Remote`
      (`self.CL_VariableFlush`))))

(event `CL_VariableFlush`
  ;[1 1 1] Variable Resets
  (if (`self.IsLocalController`)
    (`Widget.SetVisibility` (`self.ReaderWidget`) "Hidden")
    (`Widget.SetVisibility` (`self.DoBetterWidget`) "Hidden"))
  (set `self.SelectionPhase?` false)
  (set `self.CardCzar?` false)
  (set `self.CardLimitReached?` false)
  (set `self.CardsPlayed` 0)
  (`self.SR_VariableFlush`))

(event `SR_VariableFlush`
  ;[1 1 1] Variable Resets
  (if (`self.IsLocalController`)
    (`Widget.SetVisibility` (`self.ReaderWidget`) "Hidden")
    (`Widget.SetVisibility` (`self.DoBetterWidget`) "Hidden"))
  (set `self.SelectionPhase?` false)
  (set `self.CardCzar?` false)
  (set `self.CardLimitReached?` false)
  (set `self.CardsPlayed` 0)
  (`/Game/Blueprints/GameModes-Controller/MainGame/Pawn_MainGameCamera.Pawn_VariableFlush` (`self.ControlledPawn`)))

(event `MC_VariableFlush`
  ;[1 1 1] Variable Resets
  (if (`self.IsLocalController`)
    (`Widget.SetVisibility` (`self.ReaderWidget`) "Hidden")
    (`Widget.SetVisibility` (`self.DoBetterWidget`) "Hidden"))
  (set `self.SelectionPhase?` false)
  (set `self.CardCzar?` false)
  (set `self.CardLimitReached?` false)
  (set `self.CardsPlayed` 0)
  (`/Game/Blueprints/GameModes-Controller/MainGame/Pawn_MainGameCamera.Pawn_VariableFlush` (`self.ControlledPawn`)))

(fn `UserConstructionScript`)