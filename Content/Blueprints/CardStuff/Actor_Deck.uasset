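; Deck actor for a black-card party game that spawns and destroys the black card and sets the layout for player-chosen cards.
; A looping timer after BeginPlay waits for GM_Main to validate all players, then caches the deck location and picks two- and three-card layouts by player count.
; Each round, DetermineArrangement selects a layout by answer count, offsets it by the deck location and passes it to GS_Main for replication.
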(event `self.ReceiveBeginPlay`
  (bind _returnvalue (`KismetSystemLibrary.K2_SetTimerDelegate` (`|CreateDelegate` :!event `BeginPlay_Validation`) 0.1 true))
  (set `self.BeginPlayTimer` _returnvalue))

(event `BeginPlay_Validation`
  (bind _asgm_main (cast `/Game/Blueprints/GameModes-Controller/MainGame/GM_Main` (`GameplayStatics.GetGameMode`)))
  (if (and (`/Game/Blueprints/GameModes-Controller/MainGame/GM_Main.AllPawnsPossessed?` _asgm_main) (`/Game/Blueprints/GameModes-Controller/MainGame/GM_Main.AllPlayersValid?` _asgm_main))
    (`KismetSystemLibrary.K2_ClearAndInvalidateTimerHandle` (`self.BeginPlayTimer`))
    (set `self.DeckLocation` (`self.K2_GetActorLocation`))
    (bind _asgm_main_2 (cast `/Game/Blueprints/GameModes-Controller/MainGame/GM_Main` (`GameplayStatics.GetGameMode`)))
    (`self.ArrangementPrep` (`/Game/Blueprints/GameModes-Controller/MainGame/GM_Main.PlayerCount` _asgm_main_2))))

(event `ArrangementPrep`
  (params (`Player Count` :type Integer))
  (switch `int` `Player Count` ; Takes total players and decides\nwhich coordinate configuration\nto use for organizing \nplayer-chosen cards
    (:`3`
      (set `self.Active2Card` (`self.2Card1Row`))
      (set `self.Active3Card` (`self.3Card1Row`)))
    (:`4`
      (set `self.Active2Card` (`self.2Card1Row`))
      (set `self.Active3Card` (`self.3Card2Row`)))
    (:`5`
      (set `self.Active2Card` (`self.2Card2Row`))
      (set `self.Active3Card` (`self.3Card2Row`)))
    (:`6`
      (set `self.Active2Card` (`self.2Card2Row`))
      (set `self.Active3Card` (`self.3Card3Row`)))))

(event `SpawnBlackCard`
  (params (BlackCardText :type Text))
  (bind _returnvalue (`|SpawnActorFromClass` "/Game/Blueprints/CardStuff/Actor_BlackCard_Child.Actor_BlackCard_Child_C" (`KismetMathLibrary.MakeTransform` (+ (`self.DeckLocation`) (`self.BlackCardLocation`)) (`self.RotationCorrection`)) "Undefined" "OverrideRootScale" null "Actor_Card Input" true true null))
  (set `/Game/Blueprints/CardStuff/MainMenuCards/Actor_Card.TextInput` BlackCardText _returnvalue)
  (`/Game/Blueprints/CardStuff/Actor_BlackCard_Child.SendText` _returnvalue)
  (set `self.BlackCardMeshRef` _returnvalue))

(event `DetermineArrangement`
  (params (GS_AnswerCount :type Byte))
  (bind _activearrangement (`self.ActiveArrangement`))
  (switch `int` (`KismetMathLibrary.Conv_ByteToInt` GS_AnswerCount)
    (:`1`
      (set `self.ActiveArrangement` (`self.1Card`)))
    (:`2`
      (set `self.ActiveArrangement` (`self.Active2Card`)))
    (:`3`
      (set `self.ActiveArrangement` (`self.Active3Card`))))
  (for (_array_element _array_index) _activearrangement
    (`KismetArrayLibrary.Array_Set` _activearrangement _array_index (+ _array_element (`self.DeckLocation`))))
  (bind _asgs_main (cast `/Game/Blueprints/GameModes-Controller/MainGame/GS_Main` (`GameplayStatics.GetGameState`)))
  (set `/Game/Blueprints/GameModes-Controller/MainGame/GS_Main.CardArrangement` (`self.ActiveArrangement`) _asgs_main) ; Sends the arrangement for the round\nto the GS for replication
)

(event `DestroyBlackCard`
  (`self.K2_DestroyActor` (`self.BlackCardMeshRef`)))

(fn `UserConstructionScript`)