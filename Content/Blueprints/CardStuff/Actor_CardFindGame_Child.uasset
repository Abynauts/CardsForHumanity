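; Child card actor that acts as a draggable "find game" control, showing an arrow plane on hover.
; While held, a short Delay loop moves the card vertically with the deprojected mouse and clamps the cursor horizontally so the release event still fires.
; Lifting it past a height threshold fires the join camera-move dispatcher and searches online sessions, filling a join-match widget on success.
; Release or search success lerps the card back to its original location via a timeline.
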(event `self.ReceiveBeginPlay`
  (`parent.ReceiveBeginPlay`)
  (set `self.OriginalCardLocation` (`SceneComponent.K2_GetComponentLocation` (`self.StaticMesh`))))

(event `self.Widget.OnBeginCursorOver`
  (params (TouchedComponent :type "PrimitiveComponent Object Reference"))
  (if (`self.CanMouseOverCard`)
    (`SceneComponent.SetVisibility` (`self.ArrowPlane`) true false)))

(event `self.Widget.OnEndCursorOver`
  (params (TouchedComponent :type "PrimitiveComponent Object Reference"))
  (if (`self.CanMouseOverCard`)
    (`SceneComponent.SetVisibility` (`self.ArrowPlane`) false false)))

(event `self.Widget.OnClicked`
  (params (TouchedComponent :type "PrimitiveComponent Object Reference") (ButtonPressed :type "Key Structure"))
  (bind _returnvalue (`GameplayStatics.GetPlayerController` 0))
  (bind _leftsideofcard (`self.LeftSideOfCard`))
  (bind _rightsideofcard (`self.RightSideOfCard`))
  (bind _staticmesh (`self.StaticMesh`))
  (bind (_returnvalue_x _returnvalue_y _returnvalue_z) (`KismetMathLibrary.BreakVector` (`SceneComponent.K2_GetComponentLocation` _staticmesh)))
  (bind (_returnvalue_x_2 _returnvalue_y_2 _returnvalue_z_2) (`KismetMathLibrary.BreakVector` (`SceneComponent.K2_GetComponentLocation` (`self.StaticMesh`))))
  (bind (_worldlocation _worlddirection) (`PlayerController.DeprojectMousePositionToWorld` (`GameplayStatics.GetPlayerController` 0)))
  (bind (_locationx _locationy) (`PlayerController.GetMousePosition` (`GameplayStatics.GetPlayerController` 0)))
  (bind _returnvalue_2 (`KismetMathLibrary.FTrunc` _locationy))
  (bind (_returnvalue_x_3 _returnvalue_y_3 _returnvalue_z_3) (`KismetMathLibrary.BreakVector` (+ _worldlocation (* _worlddirection 120.0))))
  (set `self.IsCardClicked` true)
  (set `self.CanMouseOverCard` false)
  (`SceneComponent.SetVisibility` (`self.ArrowPlane`) false false)
  (if (`self.IsCardClicked`) :!label _label
    (`KismetSystemLibrary.Delay` 0.01)
    (set `self.CurrentCardLocation` (`KismetMathLibrary.MakeVector` _returnvalue_x _returnvalue_y _returnvalue_z))
    (`SceneComponent.K2_SetWorldLocation` _staticmesh (`KismetMathLibrary.MakeVector` _returnvalue_x 405.0 _returnvalue_z_3) false false)
    ;[1 1 1] Keeps mouse on card. If mouse isn't directly on the card, "On Released" event won't fire.
    (if (> _locationx _rightsideofcard)
      (`PlayerController.SetMouseLocation` _returnvalue (`KismetMathLibrary.FTrunc` _rightsideofcard) _returnvalue_2) ; X should be = to branch number
      (elif (< _locationx _leftsideofcard)
        (`PlayerController.SetMouseLocation` _returnvalue (`KismetMathLibrary.FTrunc` _leftsideofcard) _returnvalue_2) ; X should be = to branch number
      ))
    (if (>= _returnvalue_z_2 340.0)
      (`self.Join Camera Move Dispatcher`)
      (set `self.IsCardClicked` false)
      (bind _results (`FindSessionsCallbackProxy.FindSessions` (`GameplayStatics.GetPlayerController` 0) 100)
        (:`OnSuccess`
          (bind _returnvalue_3 (`|CreateWidget` "/Game/Networking/Widgets/Widget_JoinMatchScreen.Widget_JoinMatchScreen_C"))
          (`UserWidget.AddToViewport` _returnvalue_3 0)
          (`/Game/Networking/Widgets/Widget_JoinMatchScreen.PopulateResults` _returnvalue_3 _results)
          (set `self.IsCardClicked` false :!label _label_2)
          (set `self.CanMouseOverCard` false)
          (`KismetSystemLibrary.Delay` 0.05)
          (bind (_direction _timetoresetcard) (`Timeline|Timeline_0` :!via `PlayFromStart`)
            (:`Update`
              (`SceneComponent.K2_SetWorldLocation` (`self.StaticMesh`) (`KismetMathLibrary.VLerp` (`self.CurrentCardLocation`) (`self.OriginalCardLocation`) _timetoresetcard) false false))
            (:`Finished`
              (set `self.CanMouseOverCard` true)))))
      (else
        (goto _label)))))

(event `self.Widget.OnReleased`
  (params (TouchedComponent :type "PrimitiveComponent Object Reference") (ButtonReleased :type "Key Structure"))
  (goto _label_2))

(fn `UserConstructionScript`
  (`parent.UserConstructionScript`))