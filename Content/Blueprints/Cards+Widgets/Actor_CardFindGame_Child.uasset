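; Clickable card actor, a child of a card base class, that starts finding an online match.
; On click it prints a status message and runs an internet (non-LAN) session search for the local player.
; When the search succeeds it creates the join-match screen widget, adds it to the viewport and fills it with the found sessions.
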(event `self.ReceiveBeginPlay`
  (`parent.ReceiveBeginPlay`))

(event `self.ReceiveActorOnClicked`
  (params (ButtonPressed :type "Key Structure"))
  (`KismetSystemLibrary.PrintString` "Finding Match...")
  (bind _results (`FindSessionsCallbackProxy.FindSessions` (`GameplayStatics.GetPlayerController` 0) 100)
    (:`OnSuccess`
      (bind _returnvalue (`|CreateWidget` "/Game/Networking/JoinMatchScreenWidget.JoinMatchScreenWidget_C"))
      (`UserWidget.AddToViewport` _returnvalue 0)
      (`/Game/Networking/JoinMatchScreenWidget.PopulateResults` _returnvalue _results))))

(fn `UserConstructionScript`
  (`parent.UserConstructionScript`))