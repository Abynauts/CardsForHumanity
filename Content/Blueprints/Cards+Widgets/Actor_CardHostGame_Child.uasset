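; Clickable card actor, a child of a card base class, that hosts an online match when clicked.
; On click it prints a status message, casts the game instance to OnlineGameInstance and calls HostSession with a fixed value of six.
; It relies on the project's Game Instance Class being set to OnlineGameInstance; otherwise the cast fails and no session is hosted.
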(event `self.ReceiveActorOnClicked`
  (params (ButtonPressed :type "Key Structure"))
  ;[1 1 1] Game Instance Class must be OnlineGameInstance. We can change this in project settings - Maps & Modes
  (`KismetSystemLibrary.PrintString` "Hosting a Match...")
  (bind _asonline_game_instance (cast `/Game/Networking/OnlineMenuSystem/OnlineGameInstance` (`GameplayStatics.GetGameInstance`)))
  (`/Game/Networking/OnlineMenuSystem/OnlineGameInstance.HostSession` _asonline_game_instance 6))

(fn `UserConstructionScript`
  (`parent.UserConstructionScript`))