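; Main menu pawn that lays out the game's menu options as card actors.
; On BeginPlay it spawns host game, find game, deck builder, options and quit game cards at the transforms of alternate card slot scene components.
; The author marks this setup as placeholder code, and the construction script and other events are empty.
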(event `self.ReceiveBeginPlay`
  (`|SpawnActorFromClass` "/Game/Blueprints/Cards+Widgets/Actor_CardHostGame_Child.Actor_CardHostGame_Child_C" (`SceneComponent.K2_GetComponentToWorld` (`self.CardSlot_2`)) "Undefined" "OverrideRootScale" null null)
  (`|SpawnActorFromClass` "/Game/Blueprints/Cards+Widgets/Actor_CardFindGame_Child.Actor_CardFindGame_Child_C" (`SceneComponent.K2_GetComponentToWorld` (`self.CardSlot_4`)) "Undefined" "OverrideRootScale" null null)
  (`|SpawnActorFromClass` "/Game/Blueprints/Cards+Widgets/Actor_CardDeckBuilder_Child.Actor_CardDeckBuilder_Child_C" (`SceneComponent.K2_GetComponentToWorld` (`self.CardSlot_6`)) "Undefined" "OverrideRootScale" null null)
  (`|SpawnActorFromClass` "/Game/Blueprints/Cards+Widgets/Actor_CardOptions_Child.Actor_CardOptions_Child_C" (`SceneComponent.K2_GetComponentToWorld` (`self.CardSlot_8`)) "Undefined" "OverrideRootScale" null null)
  (`|SpawnActorFromClass` "/Game/Blueprints/Cards+Widgets/Actor_CardQuitGame_Child.Actor_CardQuitGame_Child_C" (`SceneComponent.K2_GetComponentToWorld` (`self.CardSlot_10`)) "Undefined" "OverrideRootScale" null null))

(fn `UserConstructionScript`)